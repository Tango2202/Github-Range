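; Friendly shooting-range target that swings away and deducts player score when a bullet hits it, with a larger penalty for the head than the body.
; Head and body overlaps play the Swing timeline to rotate PaperGround, set the player's Headshot flag, then destroy both hit components so it registers once.
; Head hits also show a W_Kill widget, removed after a short delay; only body hits destroy the bullet.
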(event OnComponentBeginOverlap(Head)
  (params (OverlappedComponent :type Primitive%20Component%20Object%20Reference) (OtherActor :type Actor%20Object%20Reference) (OtherComp :type Primitive%20Component%20Object%20Reference) (OtherBodyIndex :type Integer) (bFromSweep :type Boolean) (SweepResult :type Hit%20Result%20Structure%20%28by%20ref%29))
  ;[0.15 0.15 0.15 0.5] Head Overlap
  (Utilities|Casting|CastToBP_Bullet OtherActor)
  (Utilities|FlowControl|Sequence
    (:then_0
      ;[0.15 0.15 0.15 0.5] Swings using a timeline
      (bind _swingmovement (Timeline|Swing Play)
        (:Update
          (Transformation|SetRelativeRotation (Variables|Default|GetPaperGround) (Math|Rotator|Lerp(Rotator) "0, 0, 0" "-90.000000,0.000000,0.000000" _swingmovement) false false))))
    (:then_1
      (bind _asbp_player (Utilities|Casting|CastToBP_Player (Game|GetPlayerCharacter 0)))
      (Variables|/Game/Teamwork/BP/BP_Player.BP_Player_C|SetHeadshot _asbp_player true)
      (Variables|/Game/Teamwork/BP/BP_Player.BP_Player_C|SetScore _asbp_player (- (Variables|/Game/Teamwork/BP/BP_Player.BP_Player_C|GetScore _asbp_player) 15.0))
      (bind _returnvalue (UserInterface|CreateWidget "/Game/Teamwork/BP/Widget/W_Kill.W_Kill_C"))
      (UserInterface|Viewport|AddtoViewport _returnvalue 0)
      ;[0.15 0.15 0.15 0.5] Disable Overlap Components when hit once
      (Components|DestroyComponent (Variables|Default|GetHead))
      (Components|DestroyComponent (Variables|Default|GetBody))
      (bind _asbp_player_2 (Utilities|Casting|CastToBP_Player (Game|GetPlayerCharacter 0)))
      (if (Variables|/Game/Teamwork/BP/BP_Player.BP_Player_C|GetHeadshot _asbp_player_2)
        (Utilities|FlowControl|Delay 1.0)
        (bind _foundwidgets (Widget|GetAllWidgetsOfClass "/Game/Teamwork/BP/Widget/W_Kill.W_Kill_C" true))
        (Widget|RemovefromParent _foundwidgets)))))

(event OnComponentBeginOverlap(Body)
  (params (OverlappedComponent :type Primitive%20Component%20Object%20Reference) (OtherActor :type Actor%20Object%20Reference) (OtherComp :type Primitive%20Component%20Object%20Reference) (OtherBodyIndex :type Integer) (bFromSweep :type Boolean) (SweepResult :type Hit%20Result%20Structure%20%28by%20ref%29))
  ;[0.15 0.15 0.15 0.5] Body Overlap
  (bind _asbp_bullet (Utilities|Casting|CastToBP_Bullet OtherActor))
  (Actor|DestroyActor _asbp_bullet)
  (Utilities|FlowControl|Sequence
    (:then_0
      ;[0.15 0.15 0.15 0.5] Swings using a timeline
      (bind _swingmovement (Timeline|Swing Play)
        (:Update
          (Transformation|SetRelativeRotation (Variables|Default|GetPaperGround) (Math|Rotator|Lerp(Rotator) "0, 0, 0" "-90.000000,0.000000,0.000000" _swingmovement) false false))))
    (:then_1
      (bind _asbp_player (Utilities|Casting|CastToBP_Player (Game|GetPlayerCharacter 0)))
      (Variables|/Game/Teamwork/BP/BP_Player.BP_Player_C|SetHeadshot _asbp_player false)
      (Variables|/Game/Teamwork/BP/BP_Player.BP_Player_C|SetScore _asbp_player (- (Variables|/Game/Teamwork/BP/BP_Player.BP_Player_C|GetScore _asbp_player) 5.0))
      ;[0.15 0.15 0.15 0.5] Disable Overlap Components when hit once
      (Components|DestroyComponent (Variables|Default|GetHead))
      (Components|DestroyComponent (Variables|Default|GetBody))
      (bind _asbp_player_2 (Utilities|Casting|CastToBP_Player (Game|GetPlayerCharacter 0)))
      (if (Variables|/Game/Teamwork/BP/BP_Player.BP_Player_C|GetHeadshot _asbp_player_2)
        (Utilities|FlowControl|Delay 1.0)
        (bind _foundwidgets (Widget|GetAllWidgetsOfClass "/Game/Teamwork/BP/Widget/W_Kill.W_Kill_C" true))
        (Widget|RemovefromParent _foundwidgets)))))

(event EventBeginPlay)

(event Collision|EventActorBeginOverlap
  (params (OtherActor :type Actor%20Object%20Reference)))

(event EventTick
  (params (DeltaSeconds :type Float%20%28single-precision%29)))

(fn ConstructionScript)