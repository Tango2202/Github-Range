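; First-person player Blueprint with pistol shooting, reload, toggle crouch and flashlight, which also sets HP and ammo and adds the W_Score widget at start.
; Firing traces from the camera, then aims a BP_Bullet from the camera and a separate BP_VisualBullet from a Sphere component at the impact point.
; Shots also spawn casings, emit AI noise and pulse a puff effect.
; Reload refills BulletCount, capped through CurrentAmmoCount with hardcoded limits.
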(event Input|EnhancedActionEvents|EnhancedInputActionIA_Fire
  (params (ActionValue :type Float%20%28double-precision%29) (ElapsedSeconds :type Float%20%28double-precision%29) (TriggeredSeconds :type Float%20%28double-precision%29) (InputAction :type Input%20Action%20Object%20Reference :default "/Game/Input/Actions/IA_Fire.IA_Fire"))
  (bind _firstpersoncamera (Variables|Default|GetFirstPersonCamera))
  (bind _firstpersoncamera_2 (Variables|Default|GetFirstPersonCamera))
  (bind _sphere (Variables|Default|GetSphere))
  (bind _returnvalue (Transformation|GetWorldLocation _sphere))
  (bind _returnvalue_2 (Transformation|GetWorldLocation _firstpersoncamera))
  (bind _returnvalue_3 (Transformation|GetWorldLocation _firstpersoncamera_2))
  ;[0.4896 0.4896 0.4896 0.5] Shoot at camera and impact point
  (:Started
    (if (Variables|Default|GetHasPistol?)
      (bind _outhit (Collision|LineTraceByChannel _returnvalue_2 (+ _returnvalue_2 (* (Math|Vector|GetForwardVector _firstpersoncamera) 8192.0)) "TraceTypeQuery1" false 0 "None"))
      (Variables|Default|SetBulletCount (- (Math|Float|Clamp(Float) (Variables|Default|GetBulletCount) (Variables|Default|GetMinBulletCount) (Variables|Default|GetMaxBulletCount)) 1.0))
      (if (>= (Variables|Default|GetBulletCount) 1.0)
        (Audio|PlaySound2D "/Game/sfx_+_textures/silenced.silenced" 1.0 1.0 0.0 0 0)
        (Game|SpawnActorfromClass "/Game/Teamwork/BP/BP_Pistol/BP/BP_Bullet.BP_Bullet_C" (Math|Transform|MakeTransform _returnvalue_3 (Math|Rotator|FindLookatRotation _returnvalue_3 (.ImpactPoint (Collision|BreakHitResult _outhit)))) "Undefined" "OverrideRootScale" 0 0)
        (Game|SpawnActorfromClass "/Game/Teamwork/BP/BP_Pistol/BP/BP_VisualBullet.BP_VisualBullet_C" (Math|Transform|MakeTransform _returnvalue (Math|Rotator|FindLookatRotation _returnvalue (.ImpactPoint (Collision|BreakHitResult _outhit)))) "Undefined" "OverrideRootScale" 0 0)
        (Game|SpawnActorfromClass "/Game/Teamwork/BP/BP_Pistol/BP/BP_Casing.BP_Casing_C" (Transformation|GetWorldTransform (Variables|Default|GetCapsule)) "AdjustIfPossibleButAlwaysSpawn" "MultiplyWithRoot" 0 0)
        (Class|Actor|MakeNoise 1.0 self (Transformation|GetActorLocation) 0.0 "None")
        (Components|Activation|Activate (Variables|Default|GetNS_BulletPuff) false)
        (Utilities|FlowControl|Delay 0.2)
        (Components|Activation|Deactivate (Variables|Default|GetNS_BulletPuff))
        (else
          (Audio|PlaySound2D "/Game/sfx_+_textures/silenced.silenced" 1.0 1.0 0.0 0 0))))))

(event Input|EnhancedActionEvents|EnhancedInputActionIA_Flashlight
  (params (ActionValue :type Float%20%28double-precision%29) (ElapsedSeconds :type Float%20%28double-precision%29) (TriggeredSeconds :type Float%20%28double-precision%29) (InputAction :type Input%20Action%20Object%20Reference :default "/Game/Input/Actions/IA_Flashlight.IA_Flashlight"))
  ;[0.15 0.15 0.15 0.5] Flashlight
  (:Started
    (Utilities|FlowControl|FlipFlop
      (:A
        (Rendering|SetVisibility (Variables|Default|GetSpotLight) true false))
      (:B
        (Rendering|SetVisibility (Variables|Default|GetSpotLight) false false)))))

(event EventTick
  (params (DeltaSeconds :type Float%20%28single-precision%29))
  ;[0.15 0.02422 0.02422 0.5] Debug
)

(event EventBeginPlay
  ;[0.15 0.15 0.15 0.5] Begin play one offs
  (Variables|Default|SetCurrent%20HP (Variables|Default|GetMax%20HP))
  (Variables|Default|SetBulletCount (Variables|Default|GetMaxBulletCount))
  (Utilities|FlowControl|Sequence
    (:then_0
      (bind _returnvalue (UserInterface|CreateWidget "/Game/Teamwork/BP/Widget/W_Score.W_Score_C"))
      (UserInterface|Viewport|AddtoViewport _returnvalue 0))))

(event Input|KeyboardEvents|1
  (params (Key :type Key%20Structure :default "None"))
  ;[0.15 0.02422 0.02422 0.5] Debug
)

(event Input|KeyboardEvents|F
  (params (Key :type Key%20Structure :default "None"))
  ;[0.15 0.02422 0.02422 0.5] Debug
)

(event Input|KeyboardEvents|LeftCtrl
  (params (Key :type Key%20Structure :default "None"))
  ;[0.15 0.15 0.15 0.5] Crouch
  (:Pressed
    (Utilities|FlowControl|DoOnce false :!label _label
      (:Completed
        (Utilities|FlowControl|FlipFlop
          (:A
            (Character|Crouch)
            (Timeline|Crouch Play
              (:Update
                (Transformation|SetRelativeLocation (Variables|Default|GetFirstPersonCamera) "-65.000000,0.000000,0.000000" false false))))
          (:B
            (Character|UnCrouch)
            (Timeline|Timeline Play
              (:Update
                (Transformation|SetRelativeLocation (Variables|Default|GetFirstPersonCamera) "0, 0, 0" false false))))))))
  (:Released
    (goto _label Reset)))

(event Input|KeyboardEvents|R
  (params (Key :type Key%20Structure :default "None"))
  ;[0.15 0.15 0.15 0.5] Reload
  (:Pressed
    (Variables|Default|SetBulletCount (+ (Math|Float|Clamp(Float) (Variables|Default|GetBulletCount) (Variables|Default|GetMinBulletCount) (Variables|Default|GetMaxBulletCount)) (Variables|Default|GetMaxBulletCount)))
    (CallFunction|CurrentAmmoCount)))

(fn ConstructionScript)

(fn CurrentAmmoCount
  (if (>= (Variables|Default|GetBulletCount) 13.0)
    (Variables|Default|SetBulletCount 11.0)))

(fn GetWeaponTargetLocation)