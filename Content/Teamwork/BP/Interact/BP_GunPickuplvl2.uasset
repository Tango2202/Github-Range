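; BP_GunPickuplvl2 is an interactable pistol pickup for the player.
; Its overlap sphere enables input and shows a W_Interact prompt while the player character is inside, removing the prompt on exit.
; On IA_Interact it sets HasPistol on BP_Player, reveals the player's pistol, adds a W_Timer widget to the viewport and destroys itself.
; Input is enabled on any overlap and never disabled.
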(event OnComponentBeginOverlap(Sphere)
  (params (OverlappedComponent :type Primitive%20Component%20Object%20Reference) (OtherActor :type Actor%20Object%20Reference) (OtherComp :type Primitive%20Component%20Object%20Reference) (OtherBodyIndex :type Integer) (bFromSweep :type Boolean) (SweepResult :type Hit%20Result%20Structure%20%28by%20ref%29))
  ;[0.15 0.15 0.15 0.5] Interaction when overlapping
  (Input|EnableInput (Game|GetPlayerController 0))
  (if (== OtherActor (Game|GetPlayerCharacter 0))
    (UserInterface|Viewport|AddtoViewport (Variables|Default|GetInteract) 0)))

(event OnComponentEndOverlap(Sphere)
  (params (OverlappedComponent :type Primitive%20Component%20Object%20Reference) (OtherActor :type Actor%20Object%20Reference) (OtherComp :type Primitive%20Component%20Object%20Reference) (OtherBodyIndex :type Integer))
  ;[0.15 0.15 0.15 0.5] Interaction when overlapping
  (if (== (Game|GetPlayerCharacter 0) OtherActor)
    (Widget|RemovefromParent (Variables|Default|GetInteract))))

(event Input|EnhancedActionEvents|EnhancedInputActionIA_Interact
  (params (ActionValue :type Float%20%28double-precision%29) (ElapsedSeconds :type Float%20%28double-precision%29) (TriggeredSeconds :type Float%20%28double-precision%29) (InputAction :type Input%20Action%20Object%20Reference :default "/Game/Input/Actions/IA_Interact.IA_Interact"))
  ;[0.15 0.15 0.15 0.5] Interaction when overlapping
  (:Started
    (bind _asbp_player (Utilities|Casting|CastToBP_Player (Game|GetPlayerCharacter 0)))
    (Variables|/Game/Teamwork/BP/BP_Player.BP_Player_C|SetHasPistol? _asbp_player true)
    (Rendering|SetVisibility (Variables|/Game/Teamwork/BP/BP_Player.BP_Player_C|GetBP_Pistol _asbp_player) true false)
    (bind _returnvalue (UserInterface|CreateWidget "/Game/Teamwork/BP/Widget/W_Timer.W_Timer_C"))
    (UserInterface|Viewport|AddtoViewport _returnvalue 0)
    (Actor|DestroyActor)))

(event EventBeginPlay
  ;[0.15 0.15 0.15 0.5] Interaction when overlapping
  (bind _returnvalue (UserInterface|CreateWidget "/Game/Teamwork/BP/Widget/W_Interact.W_Interact_C"))
  (Variables|Default|SetInteract _returnvalue))

(fn ConstructionScript)