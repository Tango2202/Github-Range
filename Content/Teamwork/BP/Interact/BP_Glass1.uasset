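; BP_Glass1 is a breakable glass pane that shatters when a BP_Bullet overlaps its Box trigger.
; On a hit it increments WindowsBroken on player 0's BP_Player and destroys the bullet.
; It then activates a Niagara effect, removes the Cube and Box components and plays a 2D breaking sound, leaving the actor itself in place.
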(event OnComponentBeginOverlap(Box)
  (params (OverlappedComponent :type Primitive%20Component%20Object%20Reference) (OtherActor :type Actor%20Object%20Reference) (OtherComp :type Primitive%20Component%20Object%20Reference) (OtherBodyIndex :type Integer) (bFromSweep :type Boolean) (SweepResult :type Hit%20Result%20Structure%20%28by%20ref%29))
  ;[0.15 0.15 0.15 0.5] Comment
  (bind _asbp_bullet (Utilities|Casting|CastToBP_Bullet OtherActor))
  (bind _asbp_player (Utilities|Casting|CastToBP_Player (Game|GetPlayerCharacter 0)))
  (Variables|/Game/Teamwork/BP/BP_Player.BP_Player_C|SetWindowsBroken _asbp_player (+ (Variables|/Game/Teamwork/BP/BP_Player.BP_Player_C|GetWindowsBroken _asbp_player) 1.0))
  (Actor|DestroyActor _asbp_bullet)
  (Components|Activation|Activate (Variables|Default|GetNiagara) false)
  (Components|DestroyComponent (Variables|Default|GetCube))
  (Components|DestroyComponent (Variables|Default|GetBox))
  (Audio|PlaySound2D "/Game/sfx_+_textures/brkglss.brkglss" 1.0 1.0 0.0 0 0))

(event EventBeginPlay)

(event Collision|EventActorBeginOverlap
  (params (OtherActor :type Actor%20Object%20Reference)))

(event EventTick
  (params (DeltaSeconds :type Float%20%28single-precision%29)))

(fn ConstructionScript)